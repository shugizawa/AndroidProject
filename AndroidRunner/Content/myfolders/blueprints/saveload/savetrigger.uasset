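; Save trigger actor that writes a checkpoint save when its Box overlap passes a player character check.
; The check compares the overlapping component (OtherComp), not the other actor, with the player character.
; It copies the trigger's own location into the ThirdPersonCharacter's Playerlocation, then stores that and the coin count in a new SaveBP object.
; That object is saved to the "ownslot" slot and a confirmation is printed.
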(event OnComponentBeginOverlap(Box)
  (params (OverlappedComponent :type Primitive%20Component%20Object%20Reference) (OtherActor :type Actor%20Object%20Reference) (OtherComp :type Primitive%20Component%20Object%20Reference) (OtherBodyIndex :type Integer) (bFromSweep :type Boolean) (SweepResult :type Hit%20Result%20Structure%20%28by%20ref%29))
  (if (== OtherComp (Game|GetPlayerCharacter 0))
    (bind _asthird_person_character (Utilities|Casting|CastToThirdPersonCharacter (Game|GetPlayerCharacter 0)))
    (bind _returnvalue (SaveGame|CreateSaveGameObject "/Game/myfolders/blueprints/saveload/saveBP.saveBP_C"))
    (bind _output_get (Variables|Default|Setreftosave _returnvalue))
    (bind _output_get_2 (Variables|/Game/ThirdPersonBP/Blueprints/ThirdPersonCharacter.ThirdPersonCharacter_C|Setplayerlocation _asthird_person_character (Transformation|GetActorLocation)))
    (Variables|/Game/myfolders/blueprints/saveload/saveBP.saveBP_C|Setlocation_save _output_get _output_get_2)
    (Variables|/Game/myfolders/blueprints/saveload/saveBP.saveBP_C|Setcoin_save _returnvalue (Variables|/Game/ThirdPersonBP/Blueprints/ThirdPersonCharacter.ThirdPersonCharacter_C|Getcoin _asthird_person_character))
    (SaveGame|SaveGametoSlot _returnvalue "ownslot")
    (Development|PrintString "game saved")))

(event EventBeginPlay)

(event Collision|EventActorBeginOverlap
  (params (OtherActor :type Actor%20Object%20Reference)))

(event EventTick
  (params (DeltaSeconds :type Float%20%28single-precision%29)))

(fn ConstructionScript)